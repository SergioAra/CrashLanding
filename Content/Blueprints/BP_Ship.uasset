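; BP_Ship is the ship Blueprint, which sets up the game's UI and handles the end of a level.
; On BeginPlay it adds the ship UI and mission-complete widgets to the viewport.
; OnLevelComplete plays the mission-complete widget's Fade animation in reverse, waits briefly, then opens the given next level or exits the game if the name is None.
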(event `self.ReceiveBeginPlay`
  (bind _returnvalue (`|CreateWidget` "/Game/UI/WBP_ShipUI.WBP_ShipUI_C"))
  (`UserWidget.AddToViewport` _returnvalue 0)
  (bind _returnvalue_2 (`|CreateWidget` "/Game/UI/WBP_MissionComplete.WBP_MissionComplete_C"))
  (`UserWidget.AddToViewport` _returnvalue_2 0))

(event `self.OnLevelComplete`
  (params (bSuccess :type Boolean) (NextLevel :type Name))
  (`UserWidget.PlayAnimation` (stale `self.ReceiveBeginPlay` _returnvalue_2) (`/Game/UI/WBP_MissionComplete.Fade` (stale `self.ReceiveBeginPlay` _returnvalue_2)) 0.0 1 "Reverse" 1.0 false)
  (`KismetSystemLibrary.Delay` 2.0)
  (if (== NextLevel "None")
    (`KismetSystemLibrary.ExecuteConsoleCommand` "exit" null)
    (else
      (`GameplayStatics.OpenLevel` NextLevel))))

(fn `UserConstructionScript`)